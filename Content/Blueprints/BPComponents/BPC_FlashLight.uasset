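; Actor component that runs the player's battery-powered flashlight, using a light reference taken from the player on Initialize.
; Toggling shows the light only if charge remains and starts a looping timer that drains the battery, with no Tick logic.
; Each drain step remaps charge to IES brightness, dimming the light at low levels and switching it off at minimum.
; AddBatteryLife restores charge within limits without refreshing brightness.
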(fn `AddBatteryLife`
  (params (Amount :type "Float (double-precision)"))
  (set `self.CurrentBatteryLevel` (`KismetMathLibrary.FClamp` (+ Amount (`self.CurrentBatteryLevel`)) (`self.MinBatteryLevel`) (`self.MaxBatteryLevel`))))

(fn `DepleteBatteryLife`
  (bind _output_get (set `self.CurrentBatteryLevel` (`KismetMathLibrary.FClamp` (- (`self.CurrentBatteryLevel`) (`self.DepletionAmount`)) (`self.MinBatteryLevel`) (`self.MaxBatteryLevel`))))
  (`self.SetIntensity`)
  (if (<= _output_get (`self.MinBatteryLevel`))
    (`SceneComponent.SetVisibility` (`self.Flashlight light`) false false)
    (`KismetSystemLibrary.K2_ClearTimer` null "DepleteBatteryLife")))

(fn `Initialize`
  (params (Player :type "/Game/Blueprints/PlayerBPs/Uni_Character Object Reference"))
  (bind _output_get (set `self.PlayerRef` Player))
  (set `self.Flashlight light` (`/Game/Blueprints/PlayerBPs/Uni_Character.Flashlight` _output_get)))

(fn `SetIntensity`
  (`LightComponent.SetIESBrightnessScale` (`self.Flashlight light`) (`KismetMathLibrary.MapRangeClamped` (`self.CurrentBatteryLevel`) (`self.MinBatteryLevel`) 20.0 0.0 3.0)))

(fn `ToggleFlashlight`
  (bind _flashlight_light (`self.Flashlight light`))
  (if (`SceneComponent.IsVisible` _flashlight_light)
    (`SceneComponent.SetVisibility` _flashlight_light false false)
    (`KismetSystemLibrary.K2_ClearTimer` null "DepleteBatteryLife")
    (elif (> (`self.CurrentBatteryLevel`) (`self.MinBatteryLevel`))
      (`self.SetIntensity`)
      (`SceneComponent.SetVisibility` _flashlight_light true false)
      (`KismetSystemLibrary.K2_SetTimer` null "DepleteBatteryLife" (`self.DepletionSpeed`) true))))