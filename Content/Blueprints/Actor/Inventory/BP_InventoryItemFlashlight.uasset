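; BP_InventoryItemFlashlight is an inventory item that recharges the player's flashlight when used.
; Its UseItem event calls AddBatteryLife on the player's BPCFlashLight component, passing the item's BatteryAmount.
; The construction script only calls the parent, and the BeginPlay, overlap and Tick events are left as disabled stubs.
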(event `self.UseItem`
  (`/Game/Blueprints/BPComponents/BPC_FlashLight.AddBatteryLife` (`/Game/Blueprints/PlayerBPs/Uni_Character.BPC_FlashLight` (`self.PlayerRef`)) (`self.BatteryAmount`)))

(fn `UserConstructionScript`
  (`parent.UserConstructionScript`))