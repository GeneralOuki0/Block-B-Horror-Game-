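; BP_Button is a puzzle button under a glass cover, unlocked by a code set on Philosopher, Woman and Head child actors.
; BeginPlay caches the three child actor references, and Tick compares their Number values to a hardcoded combination.
; A timeline swings the glass open while the code is correct and reverses otherwise.
; Interacting while correct plays a timeline that lowers the button and sets IsPressed.
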(event `self.ReceiveBeginPlay`
  (`self.initialize`))

(event `/Game/Blueprints/Interface/BPI_Interaction.Interact`
  (if (`self.IsCorrect`)
    (bind (_direction _alpha) (`Timeline|Pressed` :!via `PlayFromStart`)
      (:`Update`
        (`SceneComponent.K2_SetRelativeLocation` (`self.Button`) (`KismetMathLibrary.MakeVector` 0.0 0.0 (`KismetMathLibrary.Lerp` 0.0 -2.0 _alpha)) false false)
        (set `self.IsPressed` true)))))

(event `self.ReceiveTick`
  (params (DeltaSeconds :type "Float (single-precision)"))
  (`self.CheckCode`)
  (if (`self.IsCorrect`)
    (bind (_direction _alpha) (`Timeline|open` :!label _label)
      (:`Update`
        (`SceneComponent.K2_SetRelativeRotation` (`self.Glass`) (`KismetMathLibrary.MakeRotator` (`KismetMathLibrary.Lerp` 0.0 -90.0 _alpha)) false false)))
    (else
      (goto _label :!via `Reverse`))))

(fn `CheckCode`
  (if (and (== (`/Game/Blueprints/Actor/Interact/RotatingStatues/BP_Philosopher.Number` (`self.PhilosopherRef`)) 0) (== (`/Game/Blueprints/Actor/Interact/RotatingStatues/BP_Woman.Number` (`self.WomanRef`)) 1) (== (`/Game/Blueprints/Actor/Interact/RotatingStatues/BP_Head.Number` (`self.HeadRef`)) 1))
    (set `self.IsCorrect` true)
    (else
      (set `self.IsCorrect` false))))

(fn `initialize`
  (bind _asbp_philosopher (cast `/Game/Blueprints/Actor/Interact/RotatingStatues/BP_Philosopher` (`ChildActorComponent.ChildActor` (`self.Philosopher`))))
  (set `self.PhilosopherRef` _asbp_philosopher)
  (bind _asbp_woman (cast `/Game/Blueprints/Actor/Interact/RotatingStatues/BP_Woman` (`ChildActorComponent.ChildActor` (`self.Woman`))))
  (set `self.WomanRef` _asbp_woman)
  (bind _asbp_head (cast `/Game/Blueprints/Actor/Interact/RotatingStatues/BP_Head` (`ChildActorComponent.ChildActor` (`self.Head`))))
  (set `self.HeadRef` _asbp_head))

(fn `UserConstructionScript`)