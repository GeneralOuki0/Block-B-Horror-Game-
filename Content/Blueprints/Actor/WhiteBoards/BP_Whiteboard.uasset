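; BP_Whiteboard is an interactable whiteboard that can show a W_CoinAI widget in the world.
; Interact blends the view to the board's camera, locks movement, look and inventory, and shows the cursor.
; Click input is forwarded through a WidgetInteraction component, and a bound widget dispatcher writes digits into text blocks.
; The Return input blends back to the character and restores movement, look and inventory access.
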(event `self.ReceiveBeginPlay`
  (`self.Initialize`)
  (if (`self.HasWidget`)
    (`SceneComponent.SetVisibility` (`self.Widget`) true false)
    (bind _asw_coin_ai (cast `/Game/UMG/Whiteboard/W_CoinAI` (`WidgetComponent.GetUserWidgetObject` (`self.Widget`))))
    (set `self.W_CoinAIRef` _asw_coin_ai)))

(event `/Game/Blueprints/Interface/BPI_Interaction.Interact`
  (bind _playercontroller (`self.PlayerController`))
  (bind _playercontroller_2 (`self.PlayerController`))
  (if (and (`self.HasWidget`) (not (`/Game/Blueprints/PlayerBPs/Uni_playerController.IsInventoryOpen` _playercontroller)))
    (set `/Game/Blueprints/PlayerBPs/Uni_playerController.CanOpenInventory` false _playercontroller)
    (`PlayerController.SetViewTargetWithBlend` (`GameplayStatics.GetPlayerController` 0) (`ActorComponent.GetOwner` (`self.Camera`)) 1.0 "VTBlend_Linear" 0.0 false)
    (`CharacterMovementComponent.DisableMovement` (`Character.CharacterMovement` (`GameplayStatics.GetPlayerCharacter` 0)))
    (`Controller.SetIgnoreLookInput` (`GameplayStatics.GetPlayerController` 0) true)
    (set `/Game/Blueprints/PlayerBPs/Uni_playerController.CanOpenInventory` false _playercontroller_2)
    (`self.EnableInput` _playercontroller_2)
    (set `PlayerController.bShowMouseCursor` true _playercontroller_2)
    (add `/Game/UMG/Whiteboard/W_CoinAI.ButtonDispatcher` (`self.W_CoinAIRef`) (delegate `CustomEvent`))))

(event `EnhancedInput|/Game/Inputs/IA_Click`
  (params (ActionValue :type Boolean) (ElapsedSeconds :type "Float (double-precision)") (TriggeredSeconds :type "Float (double-precision)") (InputAction :type "InputAction Object Reference" :default "/Game/Inputs/IA_Click.IA_Click"))
  (bind _widgetinteraction (`self.WidgetInteraction`))
  (:`Triggered`
    (`WidgetInteractionComponent.PressPointerKey` _widgetinteraction "LeftMouseButton"))
  (:`Completed`
    (`WidgetInteractionComponent.ReleasePointerKey` _widgetinteraction "LeftMouseButton")))

(event `CustomEvent`
  (params (TextBlock :type "TextBlock Object Reference") (Digit :type Integer))
  (`TextBlock.SetText` TextBlock (`KismetTextLibrary.Conv_StringToText` (`KismetStringLibrary.Conv_IntToString` Digit))))

(event `ExitLockView`
  (bind _returnvalue (`GameplayStatics.GetPlayerController` 0))
  (bind _returnvalue_2 (`GameplayStatics.GetPlayerCharacter` 0))
  (bind _playercontroller (`self.PlayerController`))
  (`PlayerController.SetViewTargetWithBlend` _returnvalue _returnvalue_2 1.0 "VTBlend_Linear" 0.0 false)
  (`self.DisableInput` _returnvalue)
  (`Controller.ResetIgnoreLookInput` _returnvalue)
  (`CharacterMovementComponent.SetMovementMode` (`Character.CharacterMovement` _returnvalue_2) "MOVE_Walking" 0)
  (set `/Game/Blueprints/PlayerBPs/Uni_playerController.CanOpenInventory` true _playercontroller)
  (set `PlayerController.bShowMouseCursor` false _playercontroller))

(event `EnhancedInput|/Game/Inputs/IA_Return`
  (params (ActionValue :type Boolean) (ElapsedSeconds :type "Float (double-precision)") (TriggeredSeconds :type "Float (double-precision)") (InputAction :type "InputAction Object Reference" :default "/Game/Inputs/IA_Return.IA_Return"))
  (:`Triggered`
    (`self.ExitLockView`)))

(fn `Initialize`
  (bind _asuni_player_controller (cast `/Game/Blueprints/PlayerBPs/Uni_playerController` (`GameplayStatics.GetPlayerController` 0)))
  (set `self.PlayerController` _asuni_player_controller))

(fn `UserConstructionScript`)