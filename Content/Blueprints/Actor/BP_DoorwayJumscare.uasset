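; BP_DoorwayJumscare is a doorway jump scare actor that reveals a DarkBeing component and slides it toward an Arrow marker.
; While CalledJumpScare is true, Tick makes DarkBeing visible and moves it at constant Speed using VInterpToConstant on world locations, without sweep.
; The flag is not set within this graph, and nothing here hides DarkBeing again or resets the flag.
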(event `self.ReceiveTick`
  (params (DeltaSeconds :type "Float (single-precision)"))
  (if (`self.CalledJumpScare`)
    (`SceneComponent.SetVisibility` (`self.DarkBeing`) true false)
    (`SceneComponent.K2_SetWorldLocation` (`self.DarkBeing`) (`KismetMathLibrary.VInterpTo_Constant` (`SceneComponent.K2_GetComponentLocation` (`self.DarkBeing`)) (`SceneComponent.K2_GetComponentLocation` (`self.Arrow`)) DeltaSeconds (`self.Speed`)) false false)))

(fn `UserConstructionScript`)