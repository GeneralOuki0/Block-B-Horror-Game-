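; Interactable keypad padlock that opens when the player enters the correct code, up to four digits long.
; Interacting blends the view to the lock's camera and suspends movement, look and inventory until Return exits.
; A WidgetInteraction component forwards clicks to the W_Pad widget, whose dispatcher appends digits to W_EnteredText, clears or submits.
; A correct code swaps a case material and swings the shackle on a timeline; a wrong one plays a sound and resets.
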(event `/Game/Blueprints/Interface/BPI_Interaction.Interact`
  (bind _playercontroller (`self.PlayerController`))
  (`PlayerController.SetViewTargetWithBlend` (`GameplayStatics.GetPlayerController` 0) (`ActorComponent.GetOwner` (`self.Camera`)) 1.0 "VTBlend_Linear" 0.0 false)
  (`CharacterMovementComponent.DisableMovement` (`Character.CharacterMovement` (`GameplayStatics.GetPlayerCharacter` 0)))
  (`Controller.SetIgnoreLookInput` (`GameplayStatics.GetPlayerController` 0) true)
  (set `/Game/Blueprints/PlayerBPs/Uni_playerController.CanOpenInventory` false _playercontroller)
  (`self.EnableInput` _playercontroller)
  (set `PlayerController.bShowMouseCursor` true _playercontroller)
  (add `/Game/UMG/Padlock/W_Pad.ButtonDispatcher` (`self.As W Pad`) (delegate `ButtonDispatcher_Event`)))

(event `EnhancedInput|/Game/Inputs/IA_Click`
  (params (ActionValue :type Boolean) (ElapsedSeconds :type "Float (double-precision)") (TriggeredSeconds :type "Float (double-precision)") (InputAction :type "InputAction Object Reference" :default "/Game/Inputs/IA_Click.IA_Click"))
  (bind _widgetinteraction (`self.WidgetInteraction`))
  (:`Started`
    (`WidgetInteractionComponent.PressPointerKey` _widgetinteraction "LeftMouseButton"))
  (:`Completed`
    (`WidgetInteractionComponent.ReleasePointerKey` _widgetinteraction "LeftMouseButton")))

(event `ExitLockView`
  (bind _returnvalue (`GameplayStatics.GetPlayerCharacter` 0))
  (bind _returnvalue_2 (`GameplayStatics.GetPlayerController` 0))
  (bind _playercontroller (`self.PlayerController`))
  (`PlayerController.SetViewTargetWithBlend` _returnvalue_2 _returnvalue 1.0 "VTBlend_Linear" 0.0 false)
  (`self.DisableInput` _returnvalue_2)
  (`Controller.ResetIgnoreLookInput` _returnvalue_2)
  (`CharacterMovementComponent.SetMovementMode` (`Character.CharacterMovement` _returnvalue) "MOVE_Walking" 0)
  (set `/Game/Blueprints/PlayerBPs/Uni_playerController.CanOpenInventory` true _playercontroller)
  (set `PlayerController.bShowMouseCursor` false _playercontroller)
  (set `self.OutOfLockView?` true))

(event `ButtonDispatcher_Event`
  (params (Digit :type Integer))
  (if (`KismetStringLibrary.EqualEqual_StrStr` (`KismetStringLibrary.Conv_IntToString` Digit) "10")
    (`self.Clear Input`)
    (elif (`KismetStringLibrary.EqualEqual_StrStr` (`KismetStringLibrary.Conv_IntToString` Digit) "11")
      (`self.TryOpen`)
      (else
        (`self.SetInputText` (`KismetStringLibrary.Conv_IntToString` Digit))))))

(event `EnhancedInput|/Game/Inputs/IA_Interact`
  (params (ActionValue :type Boolean) (ElapsedSeconds :type "Float (double-precision)") (TriggeredSeconds :type "Float (double-precision)") (InputAction :type "InputAction Object Reference" :default "/Game/Inputs/IA_Interact.IA_Interact")))

(event `EnhancedInput|/Game/Inputs/IA_Return`
  (params (ActionValue :type Boolean) (ElapsedSeconds :type "Float (double-precision)") (TriggeredSeconds :type "Float (double-precision)") (InputAction :type "InputAction Object Reference" :default "/Game/Inputs/IA_Return.IA_Return"))
  (:`Triggered`
    (`self.ExitLockView`)))

(event `self.ReceiveBeginPlay`
  (`self.Initialize`))

(event `OpenLock`
  (for (_ _array_index) (`MeshComponent.GetMaterialSlotNames` (`self.Case`))
    (if (== _array_index 2)
      (`PrimitiveComponent.SetMaterial` (`self.Case`) _array_index "/Game/Assets/PadLock/Materials/Plastic_Black.Plastic_Black")
      (bind (_direction _alpha) (`Timeline|Open`)
        (:`Update`
          (`SceneComponent.K2_SetRelativeRotation` (`self.shackle`) (`KismetMathLibrary.MakeRotator` 0.0 (`KismetMathLibrary.Lerp` 0.0 -90.0 _alpha)) false false))))))

(fn `ButtonPressed`
  (params (Digit :type Integer))
  (if (`KismetStringLibrary.EqualEqual_StrStr` (`KismetStringLibrary.Conv_IntToString` Digit) "10")
    (`self.Clear Input`)
    (elif (`KismetStringLibrary.EqualEqual_StrStr` (`KismetStringLibrary.Conv_IntToString` Digit) "11")
      (`self.TryOpen`)
      (else
        (`self.SetInputText` (`KismetStringLibrary.Conv_IntToString` Digit)))))
  (return))

(fn `Clear Input`
  (bind _output_get (set `self.Inputed` ""))
  (`TextBlock.SetText` (`/Game/UMG/Padlock/W_EnteredText.InputNumber` (`self.As W Entered Text`)) (`KismetTextLibrary.Conv_StringToText` _output_get)))

(fn `GetRef`
  (returns (PadlockRef :type "/Game/Blueprints/Actor/Lock/BP_Padlock Object Reference"))
  (return self))

(fn `Initialize`
  (bind _asuni_player_controller (cast `/Game/Blueprints/PlayerBPs/Uni_playerController` (`GameplayStatics.GetPlayerController` 0)))
  (set `self.PlayerController` _asuni_player_controller)
  (bind _asuni_character (cast `/Game/Blueprints/PlayerBPs/Uni_Character` (`GameplayStatics.GetPlayerCharacter` 0)))
  (set `self.CharacterRef` _asuni_character)
  (bind _asw_entered_text (cast `/Game/UMG/Padlock/W_EnteredText` (`WidgetComponent.GetUserWidgetObject` (`self.Input`))))
  (set `self.As W Entered Text` _asw_entered_text)
  (bind _asw_pad (cast `/Game/UMG/Padlock/W_Pad` (`WidgetComponent.GetUserWidgetObject` (`self.Pad`))))
  (set `self.As W Pad` _asw_pad)
  (set `/Game/UMG/Padlock/W_Pad.ParentPadlockReference` self _asw_pad))

(fn `SetInputText`
  (params (Digit :type String))
  (bind _output_get (set `self.Inputed` (`KismetStringLibrary.GetSubstring` (`KismetStringLibrary.Concat_StrStr` (`self.Inputed`) Digit) 0 4)))
  (`TextBlock.SetText` (`/Game/UMG/Padlock/W_EnteredText.InputNumber` (`self.As W Entered Text`)) (`KismetTextLibrary.Conv_StringToText` _output_get)))

(fn `TryOpen`
  (bind _output_get (set `self.Inputed` (`KismetTextLibrary.Conv_TextToString` (`TextBlock.GetText` (`/Game/UMG/Padlock/W_EnteredText.InputNumber` (`self.As W Entered Text`))))))
  (if (`KismetStringLibrary.EqualEqual_StrStr` _output_get (`self.CorrectCode`))
    (set `self.IsCorrect` true)
    (`self.OpenLock`)
    (else
      (`GameplayStatics.PlaySound2D` "/Engine/EditorSounds/Notifications/CompileFailed.CompileFailed" 1.0 1.0 0.0 null null)
      (bind _output_get_2 (set `self.Inputed` ""))
      (`TextBlock.SetText` (`/Game/UMG/Padlock/W_EnteredText.InputNumber` (`self.As W Entered Text`)) (`KismetTextLibrary.Conv_StringToText` _output_get_2)))))

(fn `UserConstructionScript`)