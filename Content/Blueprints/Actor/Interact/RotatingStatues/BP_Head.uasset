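; BP_Head is an interactable rotating statue head that turns a quarter turn each time it is used.
; Interact calls RotateStatue, which plays a stone sliding sound and uses a timeline to yaw the mesh, with CanRotate blocking input until it finishes.
; On finish, the accumulated angle wraps after a full turn, and FIndNumber converts it to a position index, stored in Number and printed.
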(event `RotateStatue`
  (if (`self.CanRotate`)
    (set `self.CanRotate` false)
    (`GameplayStatics.PlaySoundAtLocation` "/Game/Sounds/RotatingStatues/Stone_sliding_Cue.Stone_sliding_Cue" (`SceneComponent.RelativeLocation` (`self.SM_CeilingDetail04`)) (struct) 1.0 1.0 0.0 null null null null)
    (bind (_direction _alpha) (`Timeline|Timeline` :!via `PlayFromStart`)
      (:`Update`
        (bind _returnvalue (+ (`self.DialedRotation`) (`KismetMathLibrary.Lerp` 0.0 90.0 _alpha)))
        (`SceneComponent.K2_SetRelativeRotation` (`self.SM_CeilingDetail04`) (`KismetMathLibrary.MakeRotator` 0.0 0.0 _returnvalue) false false))
      (:`Finished`
        (set `self.DialedRotation` _returnvalue)
        (if (>= (`self.DialedRotation`) 360.0)
          (set `self.DialedRotation` 0.0)
          (`SceneComponent.K2_SetRelativeRotation` (`self.SM_CeilingDetail04`) (`KismetMathLibrary.MakeRotator` 0.0) false false))
        (`self.FIndNumber`)
        (set `self.CanRotate` true)))))

(event `FIndNumber`
  (bind _output_get (set `self.Number` (`KismetMathLibrary.FTrunc` (/ (`self.DialedRotation`) 90.0))))
  (`KismetSystemLibrary.PrintString` (`KismetStringLibrary.Conv_IntToString` _output_get)))

(event `/Game/Blueprints/Interface/BPI_Interaction.Interact`
  (`self.RotateStatue`))

(fn `UserConstructionScript`)