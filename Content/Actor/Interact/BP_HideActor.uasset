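; BP_HideActor is an interactable hiding spot that moves the player character into and back out of hiding.
; Interact starts a looping per-frame timer, first disabling the player's collision and movement when entering.
; The timer slides the player at constant speed toward the HidingPosition or ExitPosition component, chosen by the player's IsHiding flag.
; On arrival it clears the timers, fires the FinishedMoving dispatcher, flips IsHiding and restores collision and walking on exit.
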(event `self.ReceiveBeginPlay`
  (bind _asuni_character (cast `/Game/Blueprints/PlayerBPs/Uni_Character` (`GameplayStatics.GetPlayerCharacter` 0)))
  (set `self.PlayerRef` _asuni_character))

(event `/Game/Blueprints/Interface/BPI_Interaction.Interact`
  (bind _playerref (`self.PlayerRef`))
  (if (`/Game/Blueprints/PlayerBPs/Uni_Character.IsHiding?` _playerref)
    (bind _returnvalue (`KismetSystemLibrary.K2_SetTimerDelegate` (delegate `MoveCharacter`) (`GameplayStatics.GetWorldDeltaSeconds`) true))
    (else
      (`self.SetActorEnableCollision` _playerref false)
      (`CharacterMovementComponent.DisableMovement` (`Character.CharacterMovement` _playerref))
      (bind _returnvalue_2 (`KismetSystemLibrary.K2_SetTimerDelegate` (delegate `MoveCharacter`) (`GameplayStatics.GetWorldDeltaSeconds`) true)))))

(event `MoveCharacter`
  (bind _playerref (`self.PlayerRef`))
  (`self.K2_SetActorTransform` _playerref (`KismetMathLibrary.MakeTransform` (`KismetMathLibrary.VInterpTo_Constant` (`self.K2_GetActorLocation` _playerref) (`SceneComponent.K2_GetComponentLocation` (select `bool` (`/Game/Blueprints/PlayerBPs/Uni_Character.IsHiding?` (`self.PlayerRef`)) :`false` (`self.HidingPosition`) :`true` (`self.ExitPosition`) :!type "SceneComponent Object Reference")) (`GameplayStatics.GetWorldDeltaSeconds`) 1000.0)) false false)
  (if (== (`self.K2_GetActorLocation` (`self.PlayerRef`)) (`SceneComponent.K2_GetComponentLocation` (select `bool` (`/Game/Blueprints/PlayerBPs/Uni_Character.IsHiding?` (`self.PlayerRef`)) :`false` (`self.HidingPosition`) :`true` (`self.ExitPosition`) :!type "SceneComponent Object Reference")) :`ErrorTolerance` 0.01)
    (`KismetSystemLibrary.K2_ClearAndInvalidateTimerHandle` (stale `/Game/Blueprints/Interface/BPI_Interaction.Interact` _returnvalue_2))
    (`KismetSystemLibrary.K2_ClearAndInvalidateTimerHandle` (stale `/Game/Blueprints/Interface/BPI_Interaction.Interact` _returnvalue))
    (`self.FinishedMoving`)))

(event `FinishedMoving`
  (bind _playerref (`self.PlayerRef`))
  (bind _playerref_2 (`self.PlayerRef`))
  (`self.FinishedMovingED`)
  (if (`/Game/Blueprints/PlayerBPs/Uni_Character.IsHiding?` (`self.PlayerRef`))
    (set `/Game/Blueprints/PlayerBPs/Uni_Character.IsHiding?` false _playerref_2)
    (`self.SetActorEnableCollision` _playerref true)
    (`CharacterMovementComponent.SetMovementMode` (`Character.CharacterMovement` _playerref) "MOVE_Walking" 0)
    (else
      (set `/Game/Blueprints/PlayerBPs/Uni_Character.IsHiding?` true _playerref_2))))

(fn `UserConstructionScript`)